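; DemoConeActor is a demo actor whose cone mesh moves up and down along the world Z axis.
; Tick accumulates elapsed time and adds a sine of it, scaled by Frequency and a fixed amplitude, to the cone's current height.
; Because the offset accumulates each frame rather than from a stored origin, the travel range depends on frame rate.
; The construction script applies the Material variable to the cone's first slot.
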(event `self.ReceiveTick`
  (params (DeltaSeconds :type "Float (single-precision)"))
  (bind _cone (`self.Cone`))
  (bind (_returnvalue_x _returnvalue_y _returnvalue_z) (`KismetMathLibrary.BreakVector` (`SceneComponent.K2_GetComponentLocation` _cone)))
  (bind _output_get (set `self.TotalSeconds` (+ DeltaSeconds (`self.TotalSeconds`))))
  (`SceneComponent.K2_SetWorldLocation` _cone (`KismetMathLibrary.MakeVector` _returnvalue_x _returnvalue_y (+ (* (`KismetMathLibrary.Sin` (* _output_get (`self.Frequency`))) 2.0) _returnvalue_z)) false false))

(fn `UserConstructionScript`
  (`PrimitiveComponent.SetMaterial` (`self.Cone`) 0 (`self.Material`)))