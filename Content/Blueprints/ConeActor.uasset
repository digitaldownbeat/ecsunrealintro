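; ConeActor is an actor whose static mesh bobs up and down continuously.
; Tick accumulates elapsed time and adds a scaled sine of it to the mesh's current world Z.
; Because the offset is added per frame without delta-time scaling, the travel distance depends on frame rate.
; The Construction Script applies the Material variable to the mesh's first material slot.
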(event `self.ReceiveTick`
  (params (DeltaSeconds :type "Float (single-precision)"))
  (bind _staticmesh (`self.StaticMesh`))
  (bind (_returnvalue_x _returnvalue_y _returnvalue_z) (`KismetMathLibrary.BreakVector` (`SceneComponent.K2_GetComponentLocation` _staticmesh)))
  (bind _output_get (set `self.totalSeconds` (+ DeltaSeconds (`self.totalSeconds`))))
  (`SceneComponent.K2_SetWorldLocation` _staticmesh (`KismetMathLibrary.MakeVector` _returnvalue_x _returnvalue_y (+ _returnvalue_z (* (`KismetMathLibrary.Sin` (* _output_get 10.0)) 0.5))) false false))

(fn `UserConstructionScript`
  (`PrimitiveComponent.SetMaterial` (`self.StaticMesh`) 0 (`self.Material`)))